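; Exit door for Level 2 that moves the player on to Level 3 once all items are collected.
; When the Player overlaps its Box trigger, it checks ItemsCompletos; if true, it resets ItemsTemp and calls LimpiarItems.
; It then sets CurrentLevel to 3 on the 2D game mode, opens Nivel_3 and hides the mouse cursor.
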(event `self.ReceiveBeginPlay`)

(event `self.ReceiveActorBeginOverlap`
  (params (OtherActor :type "Actor Object Reference")))

(event `self.ReceiveTick`
  (params (DeltaSeconds :type "Float (single-precision)")))

(event `self.Box.OnComponentBeginOverlap`
  (params (OtherActor :type "Actor Object Reference") (OtherComp :type "PrimitiveComponent Object Reference") (OtherBodyIndex :type Integer) (bFromSweep :type Boolean) (SweepResult :type "HitResult Structure (by ref)"))
  (bind _asplayer (cast `/Game/Blueprints/Player/player` OtherActor))
  (bind _completo (`/Game/Blueprints/Player/player.Items completos` _asplayer))
  (if _completo
    (set `/Game/Blueprints/Player/player.itemsTemp` 0 _asplayer)
    (`/Game/Blueprints/Player/player.Limpiar items` _asplayer)
    (bind _as2d (cast `/Game/Blueprints/2D` (`GameplayStatics.GetGameMode`)))
    (set `/Game/Blueprints/2D.currentLevel` 3 _as2d)
    (`GameplayStatics.OpenLevel` "Nivel_3")
    (set `PlayerController.bShowMouseCursor` false (`GameplayStatics.GetPlayerController` 0))))

(fn `UserConstructionScript`)