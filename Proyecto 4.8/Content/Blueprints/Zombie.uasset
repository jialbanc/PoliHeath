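; Player-controlled 2D zombie character that walks sideways using Paper2D flipbooks.
; The MoveRight axis moves it along world X, rotates the sprite to face the direction, and picks the walk or idle flipbook from velocity, using idle during vertical motion.
; Helper functions add the PantallaPrimaria HUD, fill health and energy, and deduct energy, but nothing in this file calls them.
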(event `UpdateAnimation`
  (bind _sprite (`self.Sprite`))
  (bind _x (.x (`self.GetVelocity`)))
  (bind _z (.z (`self.GetVelocity`)))
  ;[1 1 1] Update Style Animation
  (if (or (> _z 0.0) (< _z 0.0))
    (`PaperFlipbookComponent.SetFlipbook` _sprite "/Game/FlipBooks/ReposoZombie.ReposoZombie")
    (else
      (`PaperFlipbookComponent.SetFlipbook` _sprite (select `bool` (or (> _x 0.0) (< _x 0.0)) :`false` "/Game/FlipBooks/ReposoZombie.ReposoZombie" :`true` "/Game/FlipBooks/CaminaZombie.CaminaZombie" :!type "PaperFlipbook Object Reference")))))

(event `InputAxis|MoveRight`
  (params (AxisValue :type "Float (single-precision)"))
  (bind _sprite (`self.Sprite`))
  ;[1 1 1] Update Side Animation
  (`self.UpdateAnimation`)
  (if (> AxisValue 0.0)
    (`SceneComponent.K2_SetRelativeRotation` _sprite (struct) false)
    (`self.AddMovementInput` (1.0 0.0 0.0) AxisValue :!label _label)
    (elif (< AxisValue 0.0)
      (`SceneComponent.K2_SetRelativeRotation` _sprite (struct :`Yaw` 180.0) false)
      (goto _label))))

(fn `Añadir HUD en Pantalla`
  (bind _returnvalue (`|CreateWidget` "/Game/HUD/PantallaPrimaria.PantallaPrimaria_C" (`GameplayStatics.GetPlayerController` 0)))
  (`UserWidget.AddToViewport` _returnvalue 0))

(fn `Cargar Barras de Personaje`
  (set `self.Total de Energía` 100.0)
  (set `self.Total de Vida` 100.0))

(fn `Pérdida de Energía`
  (set `self.Total de Energía` (- (`self.Total de Energía`) 15.0)))

(fn `UserConstructionScript`)