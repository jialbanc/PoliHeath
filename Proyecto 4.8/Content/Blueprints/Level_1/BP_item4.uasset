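; BP_item4 is a Level 1 pickup item with a sprite and a trigger box, collected when the player touches it.
; On box overlap, if not already collected (Recogido), it casts the other actor to Player and adds its ItemDetail, flagged as collected, via AñadirItem.
; It then hides the sprite and box and marks its own ItemDetail as collected rather than destroying the actor, blocking repeat pickups.
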(event `self.ReceiveBeginPlay`)

(event `self.ReceiveActorBeginOverlap`
  (params (OtherActor :type "Actor Object Reference")))

(event `self.ReceiveTick`
  (params (DeltaSeconds :type "Float (single-precision)")))

(event `self.Box.OnComponentBeginOverlap`
  (params (OtherActor :type "Actor Object Reference") (OtherComp :type "PrimitiveComponent Object Reference") (OtherBodyIndex :type Integer) (bFromSweep :type Boolean) (SweepResult :type "HitResult Structure (by ref)"))
  (bind (_name _reference _level _index _recogido) (break `/Game/Blueprints/BP_itemStructure` (`self.itemDetail`)))
  (bind _bp_itemstructure (make `/Game/Blueprints/BP_itemStructure` _name _reference _level _index true))
  (if (not _recogido)
    (bind _asplayer (cast `/Game/Blueprints/Player/player` OtherActor))
    (`/Game/Blueprints/Player/player.Añadir Item` _asplayer _bp_itemstructure)
    (`SceneComponent.SetHiddenInGame` (`self.PaperSprite`) true false)
    (`SceneComponent.SetVisibility` (`self.Box`) false false)
    (set `self.itemDetail` _bp_itemstructure)))

(fn `UserConstructionScript`)