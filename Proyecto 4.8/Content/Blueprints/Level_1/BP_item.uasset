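; BP_item is a collectible item actor that adds itself to the player's items on touch.
; When the Box overlaps a Player and the item is not yet marked Recogido, it passes a copy of its ItemDetail struct, flagged as collected, to AñadirItem.
; It then hides the sprite and box and sets its own flag instead of destroying itself, so it cannot be picked up again.
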(event `self.ReceiveBeginPlay`)

(event `self.ReceiveActorBeginOverlap`
  (params (OtherActor :type "Actor Object Reference")))

(event `self.ReceiveTick`
  (params (DeltaSeconds :type "Float (single-precision)")))

(event `self.Box.OnComponentBeginOverlap`
  (params (OtherActor :type "Actor Object Reference") (OtherComp :type "PrimitiveComponent Object Reference") (OtherBodyIndex :type Integer) (bFromSweep :type Boolean) (SweepResult :type "HitResult Structure (by ref)"))
  (bind (_name _reference _level _index _recogido) (break `/Game/Blueprints/BP_itemStructure` (`self.itemDetail`)))
  (bind _bp_itemstructure (make `/Game/Blueprints/BP_itemStructure` _name _reference _level _index true))
  (if (not _recogido)
    (bind _asplayer (cast `/Game/Blueprints/Player/player` OtherActor))
    (`/Game/Blueprints/Player/player.Añadir Item` _asplayer _bp_itemstructure)
    (`SceneComponent.SetHiddenInGame` (`self.PaperSprite`) true false)
    (`SceneComponent.SetVisibility` (`self.Box`) false false)
    (set `self.itemDetail` _bp_itemstructure)))

(fn `UserConstructionScript`)